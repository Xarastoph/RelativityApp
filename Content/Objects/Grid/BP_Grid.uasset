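; BP_Grid is a ground grid plane that follows the player's controlled pawn.
; The construction script creates a dynamic instance of Grid_Mat on the plane, and BeginPlay caches the BP_Controller.
; Each tick the actor moves to the pawn's X and Y at zero height.
; The plane's scale and the material's GridScale parameter are both set in proportion to pawn height, so the grid grows as the pawn rises.
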(event EventBeginPlay
  (bind _asbp_controller (Utilities|Casting|CastToBP_Controller (Game|GetPlayerController 0)))
  (Variables|Default|SetController _asbp_controller))

(event EventTick
  (params (DeltaSeconds :type Float%20%28single-precision%29))
  (bind _controller (Variables|Default|GetController)
    (:then
      (Rendering|Material|SetScalarParameterValue (Variables|Default|GetMaterial) "GridScale" (* (.Z (Math|Vector|BreakVector (Transformation|GetActorLocation (Pawn|GetControlledPawn _controller)))) 0.2) :!class /Script/Engine.MaterialInstanceDynamic)
      (Transformation|SetWorldScale3D (Variables|Default|GetPlane) (Math|Conversions|ToVector(Float) (* (.Z (Math|Vector|BreakVector (Transformation|GetActorLocation (Pawn|GetControlledPawn _controller)))) 0.2)))
      (Transformation|SetActorLocation (Math|Vector|MakeVector (.X (Math|Vector|BreakVector (Transformation|GetActorLocation (Pawn|GetControlledPawn _controller)))) (.Y (Math|Vector|BreakVector (Transformation|GetActorLocation (Pawn|GetControlledPawn _controller)))) 0.0) false false))
    (:else)))

(fn ConstructionScript
  (bind _returnvalue (Rendering|Material|CreateDynamicMaterialInstance (Variables|Default|GetPlane) 0 "/Game/Objects/Grid/Grid_Mat.Grid_Mat" :!class /Script/Engine.PrimitiveComponent))
  (Variables|Default|SetMaterial _returnvalue))