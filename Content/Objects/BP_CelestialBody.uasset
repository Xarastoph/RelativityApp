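; BP_CelestialBody is a placeable celestial body that moves under simplified N-body gravity.
; While placing, it follows a Visibility trace from the player's mouse cursor.
; Initiate registers it in the player's Bodies array and enables simulation.
; Each simulated tick, SetNewPosition sums inverse-square pulls from the other bodies' masses, without a gravitational constant, then integrates velocity and position.
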(event Custom|Initiate
  (bind _player (Variables|Default|GetPlayer)
    (:then
      (Utilities|Array|Add (Variables|/Game/Objects/BP_Controller.BP_Controller_C|GetBodies _player) self)
      (bind _output_get (Variables|Default|SetbSimulate true))
      (Development|PrintString "Hello"))
    (:else)))

(event EventBeginPlay)

(event EventTick
  (params (DeltaSeconds :type Float%20%28single-precision%29))
  (bind _player (Variables|Default|GetPlayer)
    (:then
      (if (Variables|Default|GetbPlacing)
        (bind _outhit (Collision|LineTraceByChannel (.WorldPosition (Class|GameplayStatics|DeprojectScreentoWorld _player (Math|Vector2D|MakeVector2D (.LocationX (Game|Player|GetMousePosition _player)) (.LocationY (Game|Player|GetMousePosition _player))))) (+ (.WorldPosition (Class|GameplayStatics|DeprojectScreentoWorld _player (Math|Vector2D|MakeVector2D (.LocationX (Game|Player|GetMousePosition _player)) (.LocationY (Game|Player|GetMousePosition _player))))) (Math|Vector|RotateVector "40000.000000, 0, 0" (Math|Rotator|MakeRotfromX (.WorldDirection (Class|GameplayStatics|DeprojectScreentoWorld _player (Math|Vector2D|MakeVector2D (.LocationX (Game|Player|GetMousePosition _player)) (.LocationY (Game|Player|GetMousePosition _player)))))))) "TraceTypeQuery1" false 0 "None"))
        (Transformation|SetActorLocation (.Location (Collision|BreakHitResult _outhit)) false false)
        (elif (stale Custom|Initiate _output_get)
          (CallFunction|SetNewPosition DeltaSeconds))))
    (:else)))

(fn ConstructionScript)

(fn SetNewPosition
  (params (DTime :type Float%20%28single-precision%29))
  (bind _self self)
  (bind _returnvalue (Transformation|GetActorLocation _self))
  (bind _player (Variables|Default|GetPlayer)
    (:then
      (bind _output_get (LocalVariables|SetBodies (Variables|/Game/Objects/BP_Controller.BP_Controller_C|GetBodies _player)))
      (Utilities|Array|RemoveItem _output_get _self)
      (for _array_element (LocalVariables|GetBodies)
        (bind _output_get_2 (LocalVariables|SetAcceleration (+ (stale _output_get_2) (Math|Vector|RotateVector (Math|Vector|MakeVector (/ (Variables|BP_CelestialBody_C|GetMass _array_element) (Math|Float|Square (Transformation|GetDistanceTo _array_element _self))) 0.0 0.0) (Math|Rotator|FindLookatRotation _returnvalue (Transformation|GetActorLocation _array_element)))))))
      (bind _output_get_3 (Variables|Default|SetVelocity (+ (* _output_get_2 DTime) (stale _output_get_3))))
      (Transformation|SetActorLocation (+ _returnvalue (* _output_get_3 DTime)) false false))
    (:else)))